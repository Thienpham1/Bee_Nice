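; BP_AI_Base is an AI pawn base Blueprint that chases a target and plays a rifle attack montage.
; The chase moves toward the player controller, rather than its pawn, then on success attacks and repeats after a delay.
; Attack broadcasts OnAttackEnd on montage completion or interruption.
; Helpers expose the patrol route and map movement states to walk speeds, while weapon spawn-and-attach logic is left unconnected.
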(event `self.ReceiveBeginPlay`)

(event `chase_player`
  (`|AIMoveTo` self (0.0 0.0 0.0) (`GameplayStatics.GetPlayerController` 0) 150.0
    (:`OnSuccess`
      (`self.Attack`)
      (`KismetSystemLibrary.Delay` 2.0)
      (`self.chase_player`))))

(event `Attack`
  (`|PlayMontage` (`self.Mesh`) "/Game/FirstPersonArms/Animations/FP_Rifle_Shoot_Montage.FP_Rifle_Shoot_Montage"
    (:`OnCompleted`
      _)
    (:`OnInterrupted`
      _))
  (`self.OnAttackEnd`))

(event `WieldingWeapon`)

(fn `GetPatrolRoute`
  (returns (GetPatrolRoute :type "/Game/AI/AI-Brain/BP_PatrolRoute Object Reference"))
  (return (`self.PatrolRoute`)))

(fn `SetMovementSpeed`
  (params (Speed :type "/Game/AI/Enum/E_movement_Speed Enum" :default "NewEnumerator0"))
  (returns (SpeedValue :type "Float (double-precision)"))
  (bind _output_get (set `CharacterMovementComponent.MaxWalkSpeed` (select `/Game/AI/Enum/E_movement_Speed` Speed :`NewEnumerator1` 350.0 :`NewEnumerator2` 600.0 :!type "Float (single-precision)") (`self.CharacterMovement`)))
  (return _output_get))

(fn `UserConstructionScript`)
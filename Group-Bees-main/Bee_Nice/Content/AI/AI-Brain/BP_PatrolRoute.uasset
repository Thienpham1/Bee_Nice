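; BP_PatrolRoute is a patrol route for AI that supplies waypoints from the points of its PatrolRoute spline.
; It stores the current point index and returns that point's world-space location through GetSplinePointAsWorldPostion.
; IncrementPatrolRoute steps the index by a direction value that flips at the last and first points, so the route runs back and forth rather than looping.
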(event `IncrementPatrolRoute`
  (bind _output_get (set `self.PatroIndex` (+ (`self.PatroIndex`) (`self.Direction`))))
  (if (== _output_get (- (`SplineComponent.GetNumberOfSplinePoints` (`self.Patrol_route`)) 1))
    (set `self.Direction` -1)
    (elif (== (`self.PatroIndex`) 0)
      (set `self.Direction` 1))))

(fn `GetSplinePointAsWorldPostion`
  (returns (TypeLocation :type "Vector Structure"))
  (return (`SplineComponent.GetLocationAtSplinePoint` (`self.Patrol_route`) (`self.PatroIndex`) "World")))

(fn `UserConstructionScript`)